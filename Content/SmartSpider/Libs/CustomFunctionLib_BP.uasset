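; Blueprint function library of trace and pawn-bounds helpers in the SmartSpider folder.
; GetHitWithLocation line-traces against static, dynamic, pawn and vehicle objects, ignoring the querying actor, with optional debug drawing.
; Feet and head-top helpers use the movement component's UpdatedComponent bounds; feet offset along world Z, head along actor up.
; GetHitWithFeetLocation combines both, tracing from a pawn's feet along negative actor up.
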(fn `GetHitWithFeetLocation`
  (params (QueryActor :type "Actor Object Reference") (TraceDistance :type "Float (double-precision)") (Debug :type Boolean))
  (returns (OutHit :type "HitResult Structure") (ReturnValue :type Boolean))
  (locals (DebugType :type "EDrawDebugTrace Enum"))
  (bind _aspawn (cast `Pawn` QueryActor)
    (:`then`
      (bind _returnvalue (`self.GetPawnFeetLocation` _aspawn QueryActor))
      (bind (_outhit _returnvalue_2) (`self.GetHitWithLocation` QueryActor _returnvalue (- (0.0 0.0 0.0) (`Actor.GetActorUpVector` QueryActor)) TraceDistance Debug))
      (return _outhit _returnvalue_2))
    (:`CastFailed`
      (return (struct) false))))

(fn `GetHitWithLocation`
  (params (QueryActor :type "Actor Object Reference") (StartLocation :type "Vector Structure") (TraceDir :type "Vector Structure") (TraceDistance :type "Float (double-precision)") (Debug :type Boolean) (TraceColor :type "LinearColor Structure"))
  (returns (OutHit :type "HitResult Structure") (ReturnValue :type Boolean))
  (locals (DebugType :type "EDrawDebugTrace Enum"))
  (if Debug
    (set `local.DebugType` "ForOneFrame")
    (else
      (set `local.DebugType` "None")))
  (bind (_outhit _returnvalue) (`KismetSystemLibrary.LineTraceSingleForObjects` QueryActor StartLocation (+ StartLocation (* TraceDir TraceDistance)) (`|MakeArray` "ObjectTypeQuery1" "ObjectTypeQuery2" "ObjectTypeQuery3" "ObjectTypeQuery5" :!type "EObjectTypeQuery Enum") false (`|MakeArray` QueryActor) (`local.DebugType`) true TraceColor (struct :`R` 1.0 :`G` 0.941159 :`A` 1.0)))
  (return _outhit _returnvalue))

(fn `GetPawnFeetLocation`
  (params (QueryPawn :type "Pawn Object Reference"))
  (returns (ReturnValue :type "Vector Structure"))
  (bind _updatedcomponent (`MovementComponent.UpdatedComponent` (`Pawn.GetMovementComponent` QueryPawn)))
  (if (`KismetSystemLibrary.IsValid` _updatedcomponent)
    (return (- (`SceneComponent.K2_GetComponentLocation` _updatedcomponent) (`KismetMathLibrary.MakeVector` 0.0 0.0 (.z (`.BoxExtent` (`KismetSystemLibrary.GetComponentBounds` _updatedcomponent))))))
    (else
      (return (`Actor.K2_GetActorLocation` QueryPawn)))))

(fn `GetPawnFeetOffset`
  (params (QueryPawn :type "Pawn Object Reference"))
  (returns (Offset :type "Float (double-precision)"))
  (bind _updatedcomponent (`MovementComponent.UpdatedComponent` (`Pawn.GetMovementComponent` QueryPawn)))
  (if (`KismetSystemLibrary.IsValid` _updatedcomponent)
    (return (.z (`.BoxExtent` (`KismetSystemLibrary.GetComponentBounds` _updatedcomponent))))
    (else
      (return 0.0))))

(fn `GetPawnHeadTopLocation`
  (params (QueryPawn :type "Pawn Object Reference"))
  (returns (HeadTopLocation :type "Vector Structure"))
  (bind _offset (`self.GetPawnFeetOffset` QueryPawn))
  (return (+ (* (`Actor.GetActorUpVector` QueryPawn) _offset) (`Actor.K2_GetActorLocation` QueryPawn))))